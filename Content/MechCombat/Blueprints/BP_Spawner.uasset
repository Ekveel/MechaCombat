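; BP_Spawner is a placeable spawn point that creates spider mech AI enemies at its own location.
; SpawnExplosive spawns a BP_Spider_Bomb and SpawnTurret spawns a BP_Spider_Turret, each then incrementing NumberOfBots on BP_ThirdPersonGameMode.
; It has no active events of its own, so spawning happens only when those functions are called.
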(fn `SpawnExplosive`
  (`AIBlueprintHelperLibrary.SpawnAIFromClass` "/Game/ThirdPerson/Blueprints/BP_Spider_Bomb.BP_Spider_Bomb_C" null (`self.K2_GetActorLocation`) (struct) false null)
  (bind _asbp_third_person_game_mode (cast `/Game/ThirdPerson/Blueprints/BP_ThirdPersonGameMode` (`GameplayStatics.GetGameMode`)))
  (`/Engine/EditorBlueprintResources/StandardMacros.IncrementInt` (`/Game/ThirdPerson/Blueprints/BP_ThirdPersonGameMode.numberOfBots` _asbp_third_person_game_mode)))

(fn `SpawnTurret`
  (`AIBlueprintHelperLibrary.SpawnAIFromClass` "/Game/ThirdPerson/Blueprints/BP_Spider_Turret.BP_Spider_Turret_C" null (`self.K2_GetActorLocation`) (struct) false null)
  (bind _asbp_third_person_game_mode (cast `/Game/ThirdPerson/Blueprints/BP_ThirdPersonGameMode` (`GameplayStatics.GetGameMode`)))
  (`/Engine/EditorBlueprintResources/StandardMacros.IncrementInt` (`/Game/ThirdPerson/Blueprints/BP_ThirdPersonGameMode.numberOfBots` _asbp_third_person_game_mode)))

(fn `UserConstructionScript`)